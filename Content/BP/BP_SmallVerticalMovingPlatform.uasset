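; Small moving platform actor that animates two static meshes vertically.
; On BeginPlay it waits a random fraction of a second, staggering instances, then plays the VerticalMoveAnim timeline from the start.
; Each timeline update feeds its Z track into the relative location of both meshes.
; Disconnected world-offset, world-location and local-offset variants remain in the graph but never run.
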(event EventBeginPlay
  (|CallParentFunction)
  (Utilities|FlowControl|Delay (Math|Random|RandomFloat))
  (bind _z (Timeline|VerticalMoveAnim PlayFromStart)
    (:Update
      (Transformation|SetRelativeLocation (Variables|Default|GetStaticMesh) (Math|Vector|MakeVector 0.0 0.0 _z) false false)
      (Transformation|SetRelativeLocation (Variables|Default|GetStaticMesh1) (Math|Vector|MakeVector 0.0 0.0 _z) false false))))

(event Collision|EventActorBeginOverlap
  (params (OtherActor :type Actor%20Object%20Reference))
  (|CallParentFunction OtherActor) ; This node is disabled and will not be called.\nDrag off pins to build functionality.
)

(event EventTick
  (params (DeltaSeconds :type Float%20%28single-precision%29))
  (|CallParentFunction DeltaSeconds))

(fn ConstructionScript
  (|CallParentFunction))